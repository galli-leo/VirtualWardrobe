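; Puppet is a dress-up mannequin that wears clothing items and can be animated by a standard third-person or Kinect-driven AnimBP, toggled with P and K.
; Each garment layer, trousers and shoes mesh follows the Puppet mesh through master pose.
; SetClothingItem picks the slot from the item's category, then applies its mesh and a dynamic material with color and normal textures, or clears the slot for negative IDs.
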(event EventBeginPlay
  (Input|EnableInput (Game|GetPlayerController 0)))

(event EventActorBeginOverlap
  (params (OtherActor :type Actor%20Object%20Reference)))

(event EventTick
  (params (DeltaSeconds :type Float%20%28single-precision%29)))

(event Input|KeyboardEvents|K
  (params (Key :type Key%20Structure :default "AnyKey"))
  (:Pressed
    (CallFunction|SetAnimBlueprint "/Game/Mannequin/Character/Mesh/Kinect_Driven_Anim.Kinect_Driven_Anim_C")))

(event Input|KeyboardEvents|P
  (params (Key :type Key%20Structure :default "AnyKey"))
  (:Pressed
    (CallFunction|SetAnimBlueprint "/Game/Mannequin/Animations/ThirdPerson_AnimBP.ThirdPerson_AnimBP_C")))

(fn ConstructionScript
  (bind _layer0 (Variables|Default|GetLayer0))
  (bind _returnvalue (Rendering|Material|CreateDynamicMaterialInstance _layer0 0 "/Game/Blueprints/Puppet/Topmat.Topmat" :!class /Script/Engine.PrimitiveComponent))
  (bind _output_get (Variables|Default|SetCurrentClothingItemMat _returnvalue))
  (Rendering|Material|SetTextureParameterValue _output_get "FinalTexture" "/Game/Mannequin/Character/Textures/UE4_Mannequin_MAT_MASKA.UE4_Mannequin_MAT_MASKA")
  (Rendering|Material|SetMaterial _layer0 0 _output_get)
  (CallFunction|SetAnimBlueprint "/Game/Mannequin/Animations/ThirdPerson_AnimBP.ThirdPerson_AnimBP_C"))

(fn SetClothingItem
  (params (clothingItem :type Clothing%20Item%20Structure))
  (bind (_id _category _texture) (Utilities|Struct|BreakClothingItem clothingItem))
  (bind _currentclothingitemmat (Variables|Default|GetCurrentClothingItemMat))
  (Math|Integer|CompareInt _id 0
    (:>
      (CallFunction|SetSkeletalMesh clothingItem :!label _label)
      (Rendering|Material|SetTextureParameterValue _currentclothingitemmat "FinalTexture" _texture)
      (bind _texture_2 (CallFunction|GetNormalTexture clothingItem))
      (Rendering|Material|SetTextureParameterValue _currentclothingitemmat "NormalTexture" _texture_2))
    (:==
      (goto _label))
    (:<
      (bind _component (CallFunction|GetMeshComponent _category))
      (Class|SkinnedMeshComponent|SetSkeletalMesh _component))))

(fn SetSkeletalMesh
  (params (ClothingItem :type Clothing%20Item%20Structure))
  (bind _category (Utilities|Struct|BreakClothingItem ClothingItem))
  (Utilities|FlowControl|Sequence
    (:then_0
      (bind _returnvalue (Class|MMBlueprintFunctions|GetMeshforName (.name (Utilities|Struct|BreakCategory _category))))
      (bind _component (CallFunction|GetMeshComponent _category))
      (bind _output_get (LocalVariables|SetTargetSkeletalMesh _component))
      (Class|SkinnedMeshComponent|SetSkeletalMesh _output_get _returnvalue))
    (:then_1
      (bind _returnvalue_2 (Rendering|Material|CreateDynamicMaterialInstance (LocalVariables|GetTargetSkeletalMesh) 0 "/Game/Blueprints/Puppet/Topmat.Topmat" :!class /Script/Engine.PrimitiveComponent))
      (bind _output_get_2 (Variables|Default|SetCurrentClothingItemMat _returnvalue_2)))
    (:then_2
      (Rendering|Material|SetMaterial (LocalVariables|GetTargetSkeletalMesh) 0 _output_get_2))
    (:then_3
      (CallFunction|SetAnimBlueprint "/Game/Mannequin/Animations/ThirdPerson_AnimBP.ThirdPerson_AnimBP_C"))))

(fn GetNormalTexture
  (params (Clothing%20Item :type Clothing%20Item%20Structure))
  (switch string (.name (Utilities|Struct|BreakCategory (.category (Utilities|Struct|BreakClothingItem Clothing%20Item))))
    (:tshirt
      (return "/Game/Clothes/tshirt_normal.tshirt_normal"))
    (:hoodie
      (return "/Game/Clothes/hoodie_normal.hoodie_normal"))
    (:trousers
      (return "/Game/Clothes/trousers_normal.trousers_normal"))
    (:shoes
      (return "/Game/Clothes/shoes_normal.shoes_normal"))
    (:jeans
      (return "/Game/Clothes/trousers_normal.trousers_normal"))
    (:shorts
      (return "/Game/Clothes/shorts_normal.shorts_normal"))))

(fn SetAnimBlueprint
  (params (Anim :type Anim%20Instance%20Class%20Reference))
  (bind _puppet (Variables|Default|GetPuppet))
  (Components|SkeletalMesh|SetAnimInstanceClass _puppet Anim)
  (Class|SkinnedMeshComponent|SetMasterPoseComponent (Variables|Default|GetLayer0) _puppet)
  (Class|SkinnedMeshComponent|SetMasterPoseComponent (Variables|Default|GetLayer1) _puppet)
  (Class|SkinnedMeshComponent|SetMasterPoseComponent (Variables|Default|GetTrousers) _puppet)
  (Class|SkinnedMeshComponent|SetMasterPoseComponent (Variables|Default|GetShoes) _puppet))

(fn GetMeshComponent
  (params (Category :type Category%20Structure))
  (bind (_fullname _id _name _istrousers _layer) (Utilities|Struct|BreakCategory Category))
  (Utilities|FlowControl|Sequence
    (:then_0
      (if _istrousers
        (LocalVariables|SetTarget%20Skeletal%20Mesh (Variables|Default|GetTrousers))
        (else
          (switch int _layer
            (:-1
              (LocalVariables|SetTarget%20Skeletal%20Mesh (Variables|Default|GetShoes)))
            (:0
              (LocalVariables|SetTarget%20Skeletal%20Mesh (Variables|Default|GetLayer0)))
            (:1
              (LocalVariables|SetTarget%20Skeletal%20Mesh (Variables|Default|GetLayer1)))))))
    (:then_1
      (return (LocalVariables|GetTarget%20Skeletal%20Mesh)))))
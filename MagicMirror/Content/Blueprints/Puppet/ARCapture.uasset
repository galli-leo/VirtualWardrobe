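; ARCapture is an actor that pairs a camera with a child Puppet, set up as an invisible-skinned, Kinect-driven body, apparently for AR capture.
; The construction script and BeginPlay both cast the child actor to Puppet, assign the Kinect anim blueprint and hide its skin; a SetAnim function repeats this setup.
; Inc_Height and Dec_Height inputs nudge the camera's relative height up or down in fixed steps.
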(event EventBeginPlay
  (bind _aspuppet (Utilities|Casting|CastToPuppet (Variables|/Script/Engine.ChildActorComponent|GetChildActor (Variables|Default|GetPuppet))))
  (Default|SetAnimBlueprint _aspuppet "/Game/Mannequin/Character/Mesh/Kinect_Driven_Anim.Kinect_Driven_Anim_C")
  (Default|SetSkinInvisible _aspuppet))

(event EventActorBeginOverlap
  (params (OtherActor :type Actor%20Object%20Reference)))

(event EventTick
  (params (DeltaSeconds :type Float%20%28single-precision%29)))

(event Input|ActionEvents|InputActionInc_Height
  (params (Key :type Key%20Structure :default "AnyKey"))
  (bind _camera (Variables|Default|GetCamera))
  (bind _relativelocation (Variables|/Script/Engine.SceneComponent|GetRelativeLocation _camera))
  (:Pressed
    (Transformation|SetRelativeLocation _camera (Math|Vector|MakeVector (.x _relativelocation) (.y _relativelocation) (+ (.z _relativelocation) 2.5)) false false)
    (Development|PrintString "Hello")))

(event Input|ActionEvents|InputActionDec_Height
  (params (Key :type Key%20Structure :default "AnyKey"))
  (bind _camera (Variables|Default|GetCamera))
  (bind _relativelocation (Variables|/Script/Engine.SceneComponent|GetRelativeLocation _camera))
  (:Pressed
    (Transformation|SetRelativeLocation _camera (Math|Vector|MakeVector (.x _relativelocation) (.y _relativelocation) (+ (.z _relativelocation) -2.5)) false false)))

(fn ConstructionScript
  (bind _aspuppet (Utilities|Casting|CastToPuppet (Variables|/Script/Engine.ChildActorComponent|GetChildActor (Variables|Default|GetPuppet))))
  (Default|SetAnimBlueprint _aspuppet "/Game/Mannequin/Character/Mesh/Kinect_Driven_Anim.Kinect_Driven_Anim_C")
  (Default|SetSkinInvisible _aspuppet))

(fn SetAnim
  (bind _aspuppet (Utilities|Casting|CastToPuppet (Variables|/Script/Engine.ChildActorComponent|GetChildActor (Variables|Default|GetPuppet))))
  (Default|SetAnimBlueprint _aspuppet "/Game/Mannequin/Character/Mesh/Kinect_Driven_Anim.Kinect_Driven_Anim_C")
  (Default|SetSkinInvisible _aspuppet))